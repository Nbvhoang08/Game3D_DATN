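; Test chair actor that bobs up and down continuously around the location where play begins.
; BeginPlay stores the starting location, and Tick accumulates delta time into a running timer.
; Each frame it sets the actor's Z offset from a sine of that timer, scaled by the Speed and Height variables, without sweeping.
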(event EventBeginPlay
  (Variables|Default|SetBeginLocation (Transformation|GetActorLocation)))

(event EventTick
  (params (DeltaSeconds :type Float%20%28single-precision%29))
  (bind _output_get (Variables|Val|SetMulSecond (+ DeltaSeconds (Variables|Val|GetMulSecond))))
  (Transformation|SetActorLocation (+ (Variables|Default|GetBeginLocation) (Math|Vector|MakeVector 0.0 0.0 (* (Math|Trig|Sin(Radians) (* _output_get (Variables|Val|GetSpeed))) (Variables|Val|GetHeight)))) false false))

(fn ConstructionScript)